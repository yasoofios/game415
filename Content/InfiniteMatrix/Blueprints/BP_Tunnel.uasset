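; Tunnel segment for an endless-tunnel game, with a rotating holed wall that BP_Player must pass; RandomizeWall picks its mesh and roll.
; BeginPlay spawns DOMINOS at a random offset and randomly keeps or removes the SUBWAY health pickup.
; Wall overlaps damage or kill the player and set HUSSY, which blocks the score reward.
; The exit trigger awards score, has TunnelSpawner spawn another tunnel, then destroys this one.
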(event `self.ReceiveBeginPlay`
  (bind (_returnvalue_x _returnvalue_y _returnvalue_z) (`KismetMathLibrary.BreakVector` (`self.K2_GetActorLocation`)))
  (`|SpawnActorFromClass` "/Game/InfiniteMatrix/Blueprints/DOMINOS.DOMINOS_C" (`KismetMathLibrary.MakeTransform` (`KismetMathLibrary.MakeVector` (+ (`KismetMathLibrary.RandomFloatInRange` 500.0 2000.0) _returnvalue_x) (+ (`KismetMathLibrary.RandomFloatInRange` -200.0 200.0) _returnvalue_y) (+ (`KismetMathLibrary.RandomFloatInRange` -100.0 10.0) _returnvalue_z))) "Undefined" "MultiplyWithRoot" null null)
  (if (< (`KismetMathLibrary.RandomFloat`) 0.5)
    (`SceneComponent.K2_SetRelativeLocationAndRotation` (`self.SUBWAY`) (`KismetMathLibrary.MakeVector` (+ (`KismetMathLibrary.RandomFloatInRange` 200.0 1000.0) 50.0) (+ (`KismetMathLibrary.RandomFloatInRange` -300.0 200.0) 15.0) (+ (`KismetMathLibrary.RandomFloatInRange` -100.0 10.0) 50.0)) (struct :`Pitch` 1079.999999 :`Yaw` 90.000001 :`Roll` -270.0) false false)
    (else
      (`ActorComponent.K2_DestroyComponent` (`self.SUBWAY`)))))

(event `self.ReceiveTick`
  (params (DeltaSeconds :type "Float (single-precision)"))
  (`SceneComponent.K2_AddLocalRotation` (`self.WallMesh`) (`KismetMathLibrary.MakeRotator` (* DeltaSeconds (`self.RotateSpeed`))) false false))

(event `self.TriggerZone.OnComponentBeginOverlap`
  (params (OverlappedComponent :type "PrimitiveComponent Object Reference") (OtherActor :type "Actor Object Reference") (OtherComp :type "PrimitiveComponent Object Reference") (OtherBodyIndex :type Integer) (bFromSweep :type Boolean) (SweepResult :type "HitResult Structure (by ref)"))
  (bind _asbp_player (cast `/Game/InfiniteMatrix/Blueprints/BP_Player` OtherActor))
  (if (not (`self.HUSSY`))
    (set `/Game/InfiniteMatrix/Blueprints/BP_Player.Score` (+ (`/Game/InfiniteMatrix/Blueprints/BP_Player.Score` _asbp_player) 5.0) _asbp_player))
  (`/Game/InfiniteMatrix/Blueprints/BP_TunnelSpawner.SpawnTunnelAtSpawnPoint` (`self.TunnelSpawner`))
  (`self.K2_DestroyActor`))

(event `self.WallMesh.OnComponentBeginOverlap`
  (params (OverlappedComponent :type "PrimitiveComponent Object Reference") (OtherActor :type "Actor Object Reference") (OtherComp :type "PrimitiveComponent Object Reference") (OtherBodyIndex :type Integer) (bFromSweep :type Boolean) (SweepResult :type "HitResult Structure (by ref)"))
  (set `self.HUSSY` true)
  (bind _asbp_player (cast `/Game/InfiniteMatrix/Blueprints/BP_Player` OtherActor))
  (bind _returnvalue (- (`/Game/InfiniteMatrix/Blueprints/BP_Player.Health` _asbp_player) 10.0))
  (if (< _returnvalue 0.0)
    (set `/Game/InfiniteMatrix/Blueprints/BP_Player.Health` 0.0 _asbp_player)
    (set `/Game/InfiniteMatrix/Blueprints/BP_Player.IsDead` true _asbp_player)
    (`/Game/InfiniteMatrix/Blueprints/BP_Player.DisplayRestart` _asbp_player)
    (else
      (set `/Game/InfiniteMatrix/Blueprints/BP_Player.Health` _returnvalue _asbp_player))))

(event `self.SUBWAY.OnComponentBeginOverlap`
  (params (OverlappedComponent :type "PrimitiveComponent Object Reference") (OtherActor :type "Actor Object Reference") (OtherComp :type "PrimitiveComponent Object Reference") (OtherBodyIndex :type Integer) (bFromSweep :type Boolean) (SweepResult :type "HitResult Structure (by ref)"))
  (bind _asbp_player (cast `/Game/InfiniteMatrix/Blueprints/BP_Player` OtherActor))
  (bind _returnvalue (+ (`/Game/InfiniteMatrix/Blueprints/BP_Player.Health` _asbp_player) 5.0))
  (if (> _returnvalue 100.0)
    (set `/Game/InfiniteMatrix/Blueprints/BP_Player.Health` 100.0 _asbp_player)
    (else
      (set `/Game/InfiniteMatrix/Blueprints/BP_Player.Health` _returnvalue _asbp_player)))
  (`ActorComponent.K2_DestroyComponent` (`self.SUBWAY`)))

(fn `RandomizeWall`
  (`StaticMeshComponent.SetStaticMesh` (`self.WallMesh`) (select `int` (`KismetMathLibrary.RandomIntegerInRange` 0 3) :`0` "/Game/InfiniteMatrix/Meshes/SM_Hole_01.SM_Hole_01" :`1` "/Game/InfiniteMatrix/Meshes/SM_Hole_02.SM_Hole_02" :`2` "/Game/InfiniteMatrix/Meshes/SM_Hole_03.SM_Hole_03" :`3` "/Game/InfiniteMatrix/Meshes/SM_Hole_04.SM_Hole_04" :!type "StaticMesh Object Reference"))
  (`SceneComponent.K2_AddLocalRotation` (`self.WallMesh`) (`KismetMathLibrary.MakeRotator` (`KismetMathLibrary.RandomFloatInRange` 0.0 360.0)) false false))

(fn `UserConstructionScript`)